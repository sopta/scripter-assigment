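; A learning trigger box that lets the player toggle a referenced point light's visibility with the F key while inside its volume.
; Begin and end overlap on the collision component enable and disable input for player controller 0, without checking which actor overlaps.
; On BeginPlay it also calls InteractMessage on the light.
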(event OnComponentBeginOverlap(CollisionComponent)
  (params (OverlappedComponent :type Primitive%20Component%20Object%20Reference) (OtherActor :type Actor%20Object%20Reference) (OtherComp :type Primitive%20Component%20Object%20Reference) (OtherBodyIndex :type Integer) (bFromSweep :type Boolean) (SweepResult :type Hit%20Result%20Structure%20%28by%20ref%29))
  ;[0.8048 1 0.4297 1 20] Toggle Light visibility based on the Player´s input
  (Input|EnableInput (Game|GetPlayerController 0)))

(event OnComponentEndOverlap(CollisionComponent)
  (params (OverlappedComponent :type Primitive%20Component%20Object%20Reference) (OtherActor :type Actor%20Object%20Reference) (OtherComp :type Primitive%20Component%20Object%20Reference) (OtherBodyIndex :type Integer))
  ;[0.8048 1 0.4297 1 20] Toggle Light visibility based on the Player´s input
  (Input|DisableInput (Game|GetPlayerController 0)))

(event EventBeginPlay
  (Class|BPIInteractable|Interact(Message) (Variables|Default|GetPointLight)))

(event Collision|EventActorBeginOverlap
  (params (OtherActor :type Actor%20Object%20Reference)))

(event EventTick
  (params (DeltaSeconds :type Float%20%28single-precision%29)))

(event Input|KeyboardEvents|F
  (params (Key :type Key%20Structure :default "None"))
  ;[0.8048 1 0.4297 1 20] Toggle Light visibility based on the Player´s input
  (:Pressed
    (Rendering|ToggleVisibility (Variables|/Script/Engine.Light|GetLightComponent (Variables|Default|GetPointLight)) false)))

(fn ConstructionScript)