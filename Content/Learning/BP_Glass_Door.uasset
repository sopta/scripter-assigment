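; BP_Glass_Door is an automatic sliding door that opens when the FirstPersonCharacter overlaps its Collider.
; The MoveDoors timeline lerps the Door's relative Y location to slide it open, then plays in reverse two seconds after the character leaves.
; An IsMoving flag blocks new opening triggers until the timeline finishes.
; Unconnected MoveComponentTo and Gate nodes remain unused in the graph.
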(event OnComponentBeginOverlap(collider)
  (params (OverlappedComponent :type Primitive%20Component%20Object%20Reference) (OtherActor :type Actor%20Object%20Reference) (OtherComp :type Primitive%20Component%20Object%20Reference) (OtherBodyIndex :type Integer) (bFromSweep :type Boolean) (SweepResult :type Hit%20Result%20Structure%20%28by%20ref%29))
  (if (not (Variables|Default|Getis_moving))
    (Utilities|Casting|CastToFirstPersonCharacter OtherActor)
    (Variables|Default|Setis_moving true)
    (bind _value (Timeline|Move%20doors Play)
      (:Update
        (Transformation|SetRelativeLocation (Variables|Default|Getdoor) (Math|Vector|MakeVector 0.0 (Math|Float|Lerp 0.0 -1.5e+02 _value) 0.0) false false))
      (:Finished
        (Variables|Default|Setis_moving false)))))

(event OnComponentEndOverlap(collider)
  (params (OverlappedComponent :type Primitive%20Component%20Object%20Reference) (OtherActor :type Actor%20Object%20Reference) (OtherComp :type Primitive%20Component%20Object%20Reference) (OtherBodyIndex :type Integer))
  (Utilities|Casting|CastToFirstPersonCharacter OtherActor)
  (Utilities|FlowControl|Delay 2.0)
  (bind _value (Timeline|Move%20doors Reverse)
    (:Update
      (Transformation|SetRelativeLocation (Variables|Default|Getdoor) (Math|Vector|MakeVector 0.0 (Math|Float|Lerp 0.0 -1.5e+02 _value) 0.0) false false))
    (:Finished
      (Variables|Default|Setis_moving false))))

(fn ConstructionScript)